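; Base enemy actor that chases the player, tracks its health and dies, with empty hooks such as TickStates and ChildAnimateHurt.
; Each tick it sets an integer state from player distance, turning and moving by speed-clamped physics impulses when in range.
; Health changes flag hurt; death removes it from its parent spawner's list and destroys it after a tick countdown.
; Attack timing counts ticks, but the damage branches are empty.
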(event `self.ReceiveBeginPlay`
  (bind _asplayer (cast `/Game/res/Entities/Player/Player` (`GameplayStatics.GetPlayerPawn` 0))
    (:`then`
      (set `self.PlayerReference` _asplayer))
    (:`CastFailed`
      (`KismetSystemLibrary.PrintString` "Player Not Found" true true (struct :`R` 1.0 :`A` 1.0)))))

(event `self.ReceiveTick`
  (params (DeltaSeconds :type "Float (single-precision)"))
  (`self.TickStates`)
  (`self.FollowPlayer` DeltaSeconds)
  (`self.InflictDamage` (`self.isAttacking`))
  (bind _candie (`self.HealthChecker` 0.0))
  (`self.InitDeath` _candie)
  (`self.PawnDestroy` _candie))

(fn `ChildAnimateHurt`
  (return))

(fn `ColliderAttackAnim`
  (bind _collidervisual (`self.ColliderVisual`))
  ;[0.15 0.1381 0.0537 0.5] AttackAnimChangeMaterials
  (if (`self.isAttacking`)
    (`PrimitiveComponent.SetMaterial` _collidervisual 0 "/Game/res/Textures/EntityAttacking.EntityAttacking")
    (else
      (`PrimitiveComponent.SetMaterial` _collidervisual 0 "/Game/res/Textures/Sample_Alpha.Sample_Alpha")))
  (return))

(fn `FollowDirection`
  (params (canFollow :type Boolean))
  (bind _root (`self.root`))
  (bind _movespeed (`self.MoveSpeed`))
  (if canFollow
    ;[0.081 0.04467 0.15 0.5] Impulse To Forward Vector
    (`PrimitiveComponent.AddImpulse` _root (* (`SceneComponent.GetForwardVector` _root) (`KismetMathLibrary.MakeVector` _movespeed _movespeed)) "None" true)
    ;[0.05153 0.15 0.03138 0.5] Clamp Speed
    (bind _returnvalue (`PrimitiveComponent.GetPhysicsLinearVelocity` _root "None"))
    (`PrimitiveComponent.SetPhysicsLinearVelocity` _root (`KismetMathLibrary.ClampVectorSize` _returnvalue 0.0 350.0) false "None"))
  (return))

(fn `FollowPlayer`
  (params (Delta :type "Float (double-precision)"))
  (bind _returnvalue (`SceneComponent.K2_GetComponentLocation` (`self.root`)))
  (bind _returnvalue_2 (`SceneComponent.K2_GetComponentLocation` (`/Game/res/Entities/Player/Player.PlayerBase` (`self.PlayerReference`))))
  (bind _returnvalue_3 (`KismetMathLibrary.Abs` (`KismetMathLibrary.VSize` (- _returnvalue _returnvalue_2))))
  (bind _returnvalue_4 (>= _returnvalue_3 (`self.minDist`)))
  (bind _returnvalue_5 (<= _returnvalue_3 (`self.maxDist`)))
  ;[0.2135 0.6471 0.9531 0.5] Check IsAlive
  (if (not (`self.isDead`))
    ;[0.15 0.1201 0.05694 0.5] Look At cPlayer
    (if _returnvalue_5
      (`SceneComponent.K2_SetWorldRotation` (`self.root`) (`KismetMathLibrary.MakeRotator` 0.0 0.0 (.yaw (`KismetMathLibrary.FindLookAtRotation` _returnvalue _returnvalue_2))) false false)
      ;[0.9375 0.9375 0.9375 0.5] Entity States
      (if _returnvalue_5
        (set `self.EntityState` 1)
        (if _returnvalue_4
          (set `self.EntityState` 2)
          (else
            (set `self.EntityState` 1)))
        (else
          (set `self.EntityState` 0)))
      ;[0.04199 0.1486 0.15 0.5] Follow Direction
      (`self.FollowDirection` (and _returnvalue_4 _returnvalue_5))))
  (return))

(fn `HealthChecker`
  (params (Min :type "Float (double-precision)"))
  (returns (canDie :type Boolean))
  (bind _isdead (`self.isDead`))
  (bind _health (`self.Health`))
  ;[1 0.1094 0.1094 0.5] Check HurtTick
  (if (!= _health (`self.localHealth`))
    (set `self.localHealth` _health)
    (set `self.tickHurt` true)
    (else
      (set `self.tickHurt` false)))
  ;[0.6894 0.4593 0.9375 0.5] DeathSequence
  (if (<= (`self.Health`) Min)
    (set `self.isDead` true)
    (else
      (set `self.isDead` false)))
  ;[0 0 0 0.5] ChangeState To Death
  (if _isdead
    (set `self.EntityState` -1))
  (return _isdead))

(fn `InflictDamage`
  (params (canStartInfliction :type Boolean) (DmgFrame :type Integer) (AtkMFrames :type Integer))
  (bind _localiticks (`self.localITicks`))
  ;[0.3913 0.8741 1 0.5] Damage Ticks Update
  (if canStartInfliction
    (bind _result (`/Engine/EditorBlueprintResources/StandardMacros.IncrementInt` _localiticks)
      (:`  `
        (if (== _result DmgFrame)
          (set `self.tickDamage` true)
          (else
            (set `self.tickDamage` false)))
        (if (== _localiticks AtkMFrames)
          (set `self.localITicks` 0))))
    (else
      (set `self.localITicks` 0)))
  (for _ (`PrimitiveComponent.GetOverlappingActors` (`self.EntityDetector`) "/Game/res/Entities/Player/Player.Player_C")
    (if (`self.tickDamage`)
      _
      (else
        _))
    (return)))

(fn `InitDeath`
  (params (canDie :type Boolean))
  (bind _parentspawner (`self.ParentSpawner`))
  ;[0.9167 0.7881 0.6012 0.5] Delete Self From SpawnerList
  (if canDie
    (`KismetArrayLibrary.Array_RemoveItem` (`/Game/res/Spawners/Parent/ESpawner.EntityList` _parentspawner) self)
    (bind _result (`/Engine/EditorBlueprintResources/StandardMacros.DecrementInt` (`.Entities_10_F68B842547AC44E05BAA61AEB4CD8011` (break `/Game/res/Spawners/Parent/SpawnerAttributes` (`/Game/res/Spawners/Parent/ESpawner.Attribute` _parentspawner))))
      (:`  `
        _)))
  (return))

(fn `PawnDestroy`
  (params (canStartDying :type Boolean))
  (bind _localdticks (`self.localDTicks`))
  ;[0.9327 1 0.4735 0.5] SimpleDeath Ticks
  (if canStartDying
    (`/Engine/EditorBlueprintResources/StandardMacros.IncrementInt` _localdticks
      (:`  `
        (if (== _localdticks (`self.DeathTicks`))
          (`self.K2_DestroyActor`)))))
  (return))

(fn `TickStates`
  (return))

(fn `UserConstructionScript`)